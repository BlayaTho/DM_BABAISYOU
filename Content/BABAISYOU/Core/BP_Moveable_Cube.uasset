(event Custom|Scan_IS_Nouns
  (bind _returnvalue (Transformation|GetActorLocation))
  ;[1 1 1] Scan Nouns
  (bind _outhit (Collision|LineTraceByChannel _returnvalue (+ _returnvalue (* (Transformation|GetActorForwardVector) 1e+02)) "TraceTypeQuery1" false 0 "None" true "(R=1.000000,G=0.000000,B=0.000000,A=1.000000)" "(R=0.000000,G=1.000000,B=0.000000,A=1.000000)" 2.0))
  (Variables|IS|SetHit%20Actor_1 (.HitActor (Collision|BreakHitResult _outhit)))
  (bind _outhit_2 (Collision|LineTraceByChannel _returnvalue (+ _returnvalue (* (Transformation|GetActorRightVector) -1e+02)) "TraceTypeQuery1" false 0 "None" true "(R=1.000000,G=0.000000,B=0.000000,A=1.000000)" "(R=0.000000,G=1.000000,B=0.000000,A=1.000000)" 2.0))
  (Variables|IS|SetHit%20Actor_2 (.HitActor (Collision|BreakHitResult _outhit_2)))
  (CallFunction|VerifyNouns))

(event Custom|Verify_Nouns
  (bind _hit_actor_1 (Variables|IS|GetHit%20Actor_1))
  (bind _hit_actor_2 (Variables|IS|GetHit%20Actor_2))
  ;[1 1 1] Verify Nouns
  (Utilities|IsValid _hit_actor_1
    (:Is%20Valid
      (bind _asbp_moveable_cube (Utilities|Casting|CastToBP_Moveable_Cube _hit_actor_1))
      (Variables|IS|SetRow%20Name_UP (Variables|BP_Moveable_Cube_C|GetReference%20Name _asbp_moveable_cube)))
    (:Is%20Not%20Valid
      _))
  (Utilities|IsValid _hit_actor_2
    (:Is%20Valid
      (bind _asbp_moveable_cube_2 (Utilities|Casting|CastToBP_Moveable_Cube _hit_actor_2))
      (Variables|IS|SetRow%20Name_LEFT (Variables|BP_Moveable_Cube_C|GetReference%20Name _asbp_moveable_cube_2)))
    (:Is%20Not%20Valid
      _))
  (CallFunction|ScanISProperties))

(event Custom|Scan_IS_Properties
  (bind _returnvalue (Transformation|GetActorLocation))
  ;[1 1 1] Scan Properties
  (bind (_outhit _returnvalue_2) (Collision|LineTraceByChannel _returnvalue (+ _returnvalue (* (Transformation|GetActorForwardVector) -1e+02)) "TraceTypeQuery1" false 0 "None" true "(R=1.000000,G=0.000000,B=0.000000,A=1.000000)" "(R=0.000000,G=1.000000,B=0.000000,A=1.000000)" 2.0))
  (if _returnvalue_2
    (Variables|IS|SetHit%20Actor_1 (.HitActor (Collision|BreakHitResult _outhit))))
  (bind (_outhit_2 _returnvalue_3) (Collision|LineTraceByChannel _returnvalue (+ _returnvalue (* (Transformation|GetActorRightVector) 1e+02)) "TraceTypeQuery1" false 0 "None" true "(R=1.000000,G=0.000000,B=0.000000,A=1.000000)" "(R=0.000000,G=1.000000,B=0.000000,A=1.000000)" 2.0))
  (if _returnvalue_3
    (Variables|IS|SetHit%20Actor_2 (.HitActor (Collision|BreakHitResult _outhit_2))))
  (CallFunction|VerifyProperties))

(event Custom|Verify_Properties
  (bind _hit_actor_1 (Variables|IS|GetHit%20Actor_1))
  (bind _hit_actor_2 (Variables|IS|GetHit%20Actor_2))
  ;[1 1 1] Verify properties
  (Utilities|IsValid _hit_actor_1
    (:Is%20Valid
      (bind _asbp_moveable_cube (Utilities|Casting|CastToBP_Moveable_Cube _hit_actor_1))
      (Variables|IS|SetProperty_DOWN (Variables|BP_Moveable_Cube_C|GetProperty_TEXT _asbp_moveable_cube)))
    (:Is%20Not%20Valid
      _))
  (Utilities|IsValid _hit_actor_2
    (:Is%20Valid
      (bind _asbp_moveable_cube_2 (Utilities|Casting|CastToBP_Moveable_Cube _hit_actor_2))
      (Variables|IS|SetProperty_RIGHT (Variables|BP_Moveable_Cube_C|GetProperty_TEXT _asbp_moveable_cube_2)))
    (:Is%20Not%20Valid
      _))
  (CallFunction|EndScan))

(event Custom|EndScan
  (bind _asplayer_controller_baba (Utilities|Casting|CastToPlayerController_BABA (Game|GetPlayerController 0)))
  (Default|ChangeRules _asplayer_controller_baba (Variables|IS|GetRow%20Name_UP) (Variables|IS|GetRow%20Name_LEFT) (Variables|IS|GetProperty_DOWN) (Variables|IS|GetProperty_RIGHT)))

(event EventBeginPlay
  ;[1 1 1] Begin
  (if (Utilities|Enum|Equal(Enum) (Variables|Default|GetOperator) "NewEnumerator0")
    (Utilities|FlowControl|Delay 0.2)
    (CallFunction|ScanISNouns)))

(fn ConstructionScript
  (bind _returnvalue (Utilities|GetDataTableRow "/Game/BABAISYOU/Data/DT_Types.DT_Types" (Variables|Default|GetRow%20Name))
    (:then
      (Rendering|Material|SetMaterial (Variables|Default|GetPlane) 0 (.mat _returnvalue))
      (Variables|Default|SetisLetter? (.isletter _returnvalue))
      (Variables|Default|SetProperty_TEXT (.property_text _returnvalue))
      (Variables|Default|SetReference%20Name (.referencename _returnvalue)))))